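; BP_Interactable is an interactable actor that shows a widget while something overlaps its collider and opens a CPR puzzle on interaction.
; Interact alternates through a FlipFlop, first adding a new W_CPR_Puzzle to the viewport and showing the mouse cursor.
; The next call instead plays a timeline that writes its float output into IncreaseTime on each update.
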(event `self.Collider.OnComponentBeginOverlap`
  (params (OverlappedComponent :type "PrimitiveComponent Object Reference") (OtherActor :type "Actor Object Reference") (OtherComp :type "PrimitiveComponent Object Reference") (OtherBodyIndex :type Integer) (bFromSweep :type Boolean) (SweepResult :type "HitResult Structure (by ref)"))
  (`SceneComponent.SetVisibility` (`self.Widget`) true false))

(event `self.Collider.OnComponentEndOverlap`
  (params (OverlappedComponent :type "PrimitiveComponent Object Reference") (OtherActor :type "Actor Object Reference") (OtherComp :type "PrimitiveComponent Object Reference") (OtherBodyIndex :type Integer))
  (`SceneComponent.SetVisibility` (`self.Widget`) false false))

(event `/Game/Blueprints/InteractInterface.Interact`
  (`/Engine/EditorBlueprintResources/StandardMacros.FlipFlop`
    (:`A`
      (bind _returnvalue (`|CreateWidget` "/Game/Widgets/W_CPR_Puzzle.W_CPR_Puzzle_C"))
      (`UserWidget.AddToViewport` _returnvalue 0)
      (set `PlayerController.bShowMouseCursor` true (`GameplayStatics.GetPlayerController` 0)))
    (:`B`
      (bind (_direction _flaot) (`Timeline|Timeline_0`)
        (:`Update`
          (set `self.IncreaseTime` _flaot))))))

(fn `UserConstructionScript`)