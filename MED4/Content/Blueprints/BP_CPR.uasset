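; Interactable CPR station where the player performs chest compressions and rescue breaths on a recipient mesh, with an overlap box toggling a prompt widget.
; Interact flip-flops between snapping the character into a fixed CPR pose with look and movement locked, and restoring control.
; DoAction animates both bodies and counts compressions.
; Tick watches for thirty compressions, then a DoOnce plays the breath montage with input disabled, resetting on blend out.
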(event `self.BoxCol.OnComponentBeginOverlap`
  (params (OverlappedComponent :type "PrimitiveComponent Object Reference") (OtherActor :type "Actor Object Reference") (OtherComp :type "PrimitiveComponent Object Reference") (OtherBodyIndex :type Integer) (bFromSweep :type Boolean) (SweepResult :type "HitResult Structure (by ref)"))
  ;[1 1 1] Widget
  (`SceneComponent.SetVisibility` (`self.Widget`) true false))

(event `self.BoxCol.OnComponentEndOverlap`
  (params (OverlappedComponent :type "PrimitiveComponent Object Reference") (OtherActor :type "Actor Object Reference") (OtherComp :type "PrimitiveComponent Object Reference") (OtherBodyIndex :type Integer))
  ;[1 1 1] Widget
  (`SceneComponent.SetVisibility` (`self.Widget`) false false))

(event `/Game/Blueprints/InteractInterface.Interact`
  (bind _returnvalue (`GameplayStatics.GetPlayerController` 0))
  ;[1 1 1] Press E to enter animation - Press E to leave - Locks / unlocks camera and movement
  (`/Engine/EditorBlueprintResources/StandardMacros.FlipFlop`
    (:`A`
      (bind _returnvalue_2 (`GameplayStatics.GetActorOfClass` "/Game/ThirdPerson/Blueprints/BP_ThirdPersonCharacter.BP_ThirdPersonCharacter_C"))
      (`self.K2_SetActorLocation` _returnvalue_2 (510.0 640.0 -3.0) false false)
      (`|PlayMontage` (`Character.Mesh` _returnvalue_2) "/Game/Animations/Game/M_AdmCPR.M_AdmCPR"
        (:`then`
          (`Controller.SetIgnoreLookInput` _returnvalue true)
          (`Controller.SetIgnoreMoveInput` _returnvalue true))))
    (:`B`
      (bind _returnvalue_3 (`GameplayStatics.GetActorOfClass` "/Game/ThirdPerson/Blueprints/BP_ThirdPersonCharacter.BP_ThirdPersonCharacter_C"))
      (`SkeletalMeshComponent.SetAnimationMode` (`Character.Mesh` _returnvalue_3) "AnimationBlueprint" true)
      (`Controller.SetIgnoreLookInput` _returnvalue false)
      (`Controller.SetIgnoreMoveInput` _returnvalue false))))

(event `/Game/Blueprints/DoActionInterface.DoAction`
  (`SkeletalMeshComponent.PlayAnimation` (`self.RecCPR`) "/Game/Animations/Game/RecCPRpart.RecCPRpart" false)
  (bind _returnvalue (`GameplayStatics.GetActorOfClass` "/Game/ThirdPerson/Blueprints/BP_ThirdPersonCharacter.BP_ThirdPersonCharacter_C"))
  (`|PlayMontage` (`Character.Mesh` _returnvalue) "/Game/Animations/Game/M_AdmCPR.M_AdmCPR"
    (:`then`
      (bind _output_get (set `self.Compressions` (+ (`self.Compressions`) 1)))
      (`KismetSystemLibrary.PrintText` (`KismetTextLibrary.Conv_IntToText` _output_get)))))

(event `self.ReceiveTick`
  (params (DeltaSeconds :type "Float (single-precision)"))
  ;[1 1 1] Handles the mouth to mouth, disables all imputs while the animation is playing
  (if (== (`self.Compressions`) 30)
    (`/Engine/EditorBlueprintResources/StandardMacros.DoOnce` false :!label _label
      (:`Completed`
        (`self.DisableInput` (`GameplayStatics.GetPlayerCharacter` 0) (`GameplayStatics.GetPlayerController` 0))
        (bind _returnvalue (`GameplayStatics.GetActorOfClass` "/Game/ThirdPerson/Blueprints/BP_ThirdPersonCharacter.BP_ThirdPersonCharacter_C"))
        (`|PlayMontage` (`Character.Mesh` _returnvalue) "/Game/Animations/Game/M_Adm_Blow.M_Adm_Blow"
          (:`OnBlendOut`
            (bind _output_get (set `self.Compressions` 0))
            (`KismetSystemLibrary.PrintText` (`KismetTextLibrary.Conv_IntToText` _output_get))
            (bind _returnvalue_2 (`GameplayStatics.GetActorOfClass` "/Game/ThirdPerson/Blueprints/BP_ThirdPersonCharacter.BP_ThirdPersonCharacter_C"))
            (`self.EnableInput` (`GameplayStatics.GetPlayerCharacter` 0) (`GameplayStatics.GetPlayerController` 0))
            (`|PlayMontage` (`Character.Mesh` _returnvalue_2) "/Game/Animations/Game/M_AdmCPR.M_AdmCPR"
              (:`then`
                (goto _label :!via `Reset`)))))))))

(fn `UserConstructionScript`)