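; Lock button for the "5" key, likely one digit of a keypad, that animates and beeps when pressed.
; Box overlaps with the third-person character open and close a Gate, so the 5 key responds only while the player is in range.
; A press plays Beep5, then chained ButtonIn and reversed ButtonOut timelines lerp the Button between transforms cached at BeginPlay.
; No code entry or unlock logic is present here.
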(event `self.ReceiveBeginPlay`
  (bind (_returnvalue_location _returnvalue_rotation _returnvalue_scale) (`KismetMathLibrary.BreakTransform` (`SceneComponent.GetRelativeTransform` (`self.Button`))))
  (set `self.Out Position` (`KismetMathLibrary.MakeTransform` _returnvalue_location _returnvalue_rotation _returnvalue_scale))
  (set `self.InPosition` (`KismetMathLibrary.MakeTransform` (- _returnvalue_location _returnvalue_location (5.0 0.0 0.0)) _returnvalue_rotation _returnvalue_scale))
  (`self.EnableInput` (`GameplayStatics.GetPlayerController` 0)))

(event `Key|Five`
  (params (Key :type "Key Structure"))
  (:`Pressed`
    (`/Engine/EditorBlueprintResources/StandardMacros.Gate` true :!label _label
      (:`Exit`
        (`GameplayStatics.PlaySoundAtLocation` "/Game/Sounds/Beep5.Beep5" (`self.K2_GetActorLocation`) (struct) 1.0 1.0 0.0 null null null null)
        (bind (_direction _button_in) (`Timeline|Button In` :!via `PlayFromStart`)
          (:`Update`
            (`SceneComponent.K2_SetRelativeTransform` (`self.Button`) (`KismetMathLibrary.TLerp` (`self.Out Position`) (`self.InPosition`) _button_in) false false))
          (:`Finished`
            (bind (_direction_2 _button_in_2) (`Timeline|Button Out` :!via `ReverseFromEnd`)
              (:`Update`
                (`SceneComponent.K2_SetRelativeTransform` (`self.Button`) (`KismetMathLibrary.TLerp` (`self.Out Position`) (`self.InPosition`) _button_in_2) false false)))))))))

(event `self.Box.OnComponentBeginOverlap`
  (params (OverlappedComponent :type "PrimitiveComponent Object Reference") (OtherActor :type "Actor Object Reference") (OtherComp :type "PrimitiveComponent Object Reference") (OtherBodyIndex :type Integer) (bFromSweep :type Boolean) (SweepResult :type "HitResult Structure (by ref)"))
  (cast `/Game/ThirdPerson/Blueprints/BP_ThirdPersonCharacter` OtherActor)
  (goto _label :!via `Open`))

(event `self.Box.OnComponentEndOverlap`
  (params (OverlappedComponent :type "PrimitiveComponent Object Reference") (OtherActor :type "Actor Object Reference") (OtherComp :type "PrimitiveComponent Object Reference") (OtherBodyIndex :type Integer))
  (cast `/Game/ThirdPerson/Blueprints/BP_ThirdPersonCharacter` OtherActor)
  (goto _label :!via `Close`))

(fn `UserConstructionScript`)